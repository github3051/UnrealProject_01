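; A vector-math example actor that chases the actor in Other at a constant Speed and quits the game once it gets within Distance.
; Each Tick it normalizes the direction to Other, scales it by Speed and DeltaSeconds, and sets the new location without sweeping.
; When the gap is no longer greater than Distance, it calls QuitGame instead of moving.
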(event EventTick
  (params (DeltaSeconds :type Float%20%28single-precision%29))
  (if (> (Transformation|GetDistanceTo (Variables|Default|GetOther) self) (Variables|Default|GetDistance))
    (Transformation|SetActorLocation (+ (* (Math|Vector|Normalize (- (Transformation|GetActorLocation (Variables|Default|GetOther)) (Transformation|GetActorLocation))) (* DeltaSeconds (Variables|Default|GetSpeed))) (Transformation|GetActorLocation)) false false)
    (else
      (Game|QuitGame 0 "Quit" false))))

(fn ConstructionScript)