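; BP_02_Variable is a small test Blueprint that demonstrates variable use by printing values to the screen at BeginPlay.
; A Sequence node first stores the sum of A and B in C and prints it.
; It then prints D and E converted to text and joined into one labeled string in red.
; The construction script is empty.
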(event EventBeginPlay
  (Utilities|FlowControl|Sequence
    (:then_0
      (bind _output_get (Variables|Default|SetC (+ (Variables|Default|GetA) (Variables|Default|GetB))))
      (Development|PrintString (Utilities|String|ToString(Integer) _output_get) true true "(R=0.000000,G=0.660000,B=1.000000,A=1.000000)" 1e+01))
    (:then_1
      (Development|PrintString (Utilities|String|Append "D : " (Utilities|String|ToString(Integer) (Variables|Default|GetD)) " / " "E : " (Utilities|String|ToString(Integer) (Variables|Default|GetE))) true true "(R=1.000000,G=0.000000,B=0.000000,A=1.000000)" 1e+01))))

(fn ConstructionScript)