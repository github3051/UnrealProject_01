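; Demo actor that reports collision events on its Box component with on-screen debug text.
; Begin overlap, end overlap and hit events each print the names of the own component, the other actor and the other component.
; End overlap and hit use their own text colors to tell the event types apart.
; The construction script is empty.
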(event OnComponentBeginOverlap(Box)
  (params (OverlappedComponent :type Primitive%20Component%20Object%20Reference) (OtherActor :type Actor%20Object%20Reference) (OtherComp :type Primitive%20Component%20Object%20Reference) (OtherBodyIndex :type Integer) (bFromSweep :type Boolean) (SweepResult :type Hit%20Result%20Structure%20%28by%20ref%29))
  (Development|PrintString (Utilities|String|Append (Utilities|GetDisplayName OverlappedComponent) " / " (Utilities|GetDisplayName OtherActor) " / " (Utilities|GetDisplayName OtherComp)) true true "(R=0.000000,G=0.660000,B=1.000000,A=1.000000)" 1e+01))

(event OnComponentEndOverlap(Box)
  (params (OverlappedComponent :type Primitive%20Component%20Object%20Reference) (OtherActor :type Actor%20Object%20Reference) (OtherComp :type Primitive%20Component%20Object%20Reference) (OtherBodyIndex :type Integer))
  (Development|PrintString (Utilities|String|Append (Utilities|GetDisplayName OverlappedComponent) " / " (Utilities|GetDisplayName OtherActor) " / " (Utilities|GetDisplayName OtherComp)) true true "(R=1.000000,G=0.000000,B=1.000000,A=1.000000)" 1e+01))

(event OnComponentHit(Box)
  (params (HitComponent :type Primitive%20Component%20Object%20Reference) (OtherActor :type Actor%20Object%20Reference) (OtherComp :type Primitive%20Component%20Object%20Reference) (NormalImpulse :type Vector :default "0, 0, 0") (Hit :type Hit%20Result%20Structure%20%28by%20ref%29))
  (Development|PrintString (Utilities|String|Append (Utilities|GetDisplayName HitComponent) " / " (Utilities|GetDisplayName OtherActor) " / " (Utilities|GetDisplayName OtherComp)) true true "(R=1.000000,G=0.000000,B=0.000000,A=1.000000)" 1e+01))

(fn ConstructionScript)