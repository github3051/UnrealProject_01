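; Enemy character with health that reacts to hits and dies when health reaches zero.
; AnyDamage lowers clamped health only when the instigator controls a Character, storing it as Attacker.
; Surviving hits play a montage, flash BodyColor red via BeginPlay-created dynamic materials, face the attacker and launch backward.
; Death disables capsule collision and plays a fall montage, while a separate End_Dead event destroys the actor.
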(event Custom|Dead
  (Collision|SetCollisionEnabled (Variables|Collision|GetCapsuleComponent) "NoCollision")
  (Animation|PlayAnimMontage "/Game/Character/Montages/Common/Enemy_DeadFall_Montage.Enemy_DeadFall_Montage" 1.0 "None"))

(event Custom|End_Dead
  (Actor|DestroyActor))

(event Game|Damage|EventAnyDamage
  (params (Damage :type Float%20%28single-precision%29) (DamageType :type Damage%20Type%20Object%20Reference) (InstigatedBy :type Controller%20Object%20Reference) (DamageCauser :type Actor%20Object%20Reference))
  (|SetDamage Damage InstigatedBy
    (:Dead
      (CallFunction|Dead))
    (:Hitted
      (Animation|PlayAnimMontage "/Game/Character/Montages/Common/HitReaction_Montage.HitReaction_Montage" 2.0 "None")
      (Maerial|SetColor)
      (|LookAt)
      (|Launch))))

(event EventBeginPlay
  (Variables|Default|SetHealth (Variables|Default|GetMaxHealth))
  (for _array_element (Rendering|Material|GetMaterials (Variables|Character|GetMesh))
    (bind _returnvalue (Rendering|Material|CreateDynamicMaterialInstance _array_element "None" "None" :!class /Script/Engine.KismetMaterialLibrary))
    (bind _returnvalue_2 (Utilities|Array|Add (Variables|Default|GetMaterials) _returnvalue))
    (Rendering|Material|SetMaterial (Variables|Character|GetMesh) _returnvalue_2 _returnvalue)))

(fn ConstructionScript)